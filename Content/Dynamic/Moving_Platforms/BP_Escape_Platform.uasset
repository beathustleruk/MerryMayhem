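; BP_Escape_Platform is a moving platform tied to the player's exit-open state and to a trigger box.
; Tick polls the third-person character's IsExitOpen, then plays a one-shot timeline that sets the platform's relative location only when it finishes.
; Player overlap with the box plays a second timeline that moves the platform every update.
; That update path also feeds a five-second delay, which first reverses the timeline, then re-enters the play path once IsLooping is set.
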(event OnComponentBeginOverlap(Box)
  (params (OverlappedComponent :type Primitive%20Component%20Object%20Reference) (OtherActor :type Actor%20Object%20Reference) (OtherComp :type Primitive%20Component%20Object%20Reference) (OtherBodyIndex :type Integer) (bFromSweep :type Boolean) (SweepResult :type Hit%20Result%20Structure%20%28by%20ref%29))
  (Utilities|Casting|CastToBP_ThirdPersonCharacter OtherActor :!label _label)
  (bind _newtrack_0 (Timeline|Timeline Play)
    (:Update
      (Transformation|SetRelativeLocation (Variables|Default|GetPlatform) _newtrack_0 false false)
      (Utilities|FlowControl|Delay 5.0)
      (if (Variables|Default|GetIs%20Looping?)
        (goto _label)
        (else
          (Variables|Default|SetIs%20Looping? true)
          (Timeline|Timeline Reverse))))))

(event EventTick
  (params (DeltaSeconds :type Float%20%28single-precision%29))
  (bind _asbp_third_person_character (Utilities|Casting|CastToBP_ThirdPersonCharacter (Game|GetPlayerCharacter 0)))
  (if (Variables|/Game/Dynamic/ThirdPerson/Blueprints/BP_ThirdPersonCharacter.BP_ThirdPersonCharacter_C|GetIs%20Exit%20open? _asbp_third_person_character)
    (Utilities|FlowControl|DoOnce false
      (:Completed
        (bind _newtrack_0 (Timeline|Timeline_0 Play)
          (:Finished
            (Transformation|SetRelativeLocation (Variables|Default|GetPlatform) _newtrack_0 false false)))))))

(fn ConstructionScript)