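; BP_Candy_Cane is a candy cane collectable that rewards the player on pickup and then destroys itself.
; When its Sphere overlaps BP_ThirdPersonCharacter, it raises that character's Score and Collectables count.
; It also adds bonus seconds to the BP_ThirdPersonGameMode timer, then plays a 2D feedback sound with randomised pitch.
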(event OnComponentBeginOverlap(Sphere)
  (params (OverlappedComponent :type Primitive%20Component%20Object%20Reference) (OtherActor :type Actor%20Object%20Reference) (OtherComp :type Primitive%20Component%20Object%20Reference) (OtherBodyIndex :type Integer) (bFromSweep :type Boolean) (SweepResult :type Hit%20Result%20Structure%20%28by%20ref%29))
  ;[1 1 1] Collected
  (bind _asbp_third_person_character (Utilities|Casting|CastToBP_ThirdPersonCharacter OtherActor))
  (Variables|/Game/Dynamic/ThirdPerson/Blueprints/BP_ThirdPersonCharacter.BP_ThirdPersonCharacter_C|SetScore _asbp_third_person_character (+ (Variables|/Game/Dynamic/ThirdPerson/Blueprints/BP_ThirdPersonCharacter.BP_ThirdPersonCharacter_C|GetScore _asbp_third_person_character) 25))
  (Variables|/Game/Dynamic/ThirdPerson/Blueprints/BP_ThirdPersonCharacter.BP_ThirdPersonCharacter_C|SetCollectables _asbp_third_person_character (+ (Variables|/Game/Dynamic/ThirdPerson/Blueprints/BP_ThirdPersonCharacter.BP_ThirdPersonCharacter_C|GetCollectables _asbp_third_person_character) 1))
  (bind _asbp_third_person_game_mode (Utilities|Casting|CastToBP_ThirdPersonGameMode (Game|GetGameMode)))
  (Variables|/Game/Dynamic/ThirdPerson/Blueprints/BP_ThirdPersonGameMode.BP_ThirdPersonGameMode_C|SetTimer%20Seconds _asbp_third_person_game_mode (+ (Variables|/Game/Dynamic/ThirdPerson/Blueprints/BP_ThirdPersonGameMode.BP_ThirdPersonGameMode_C|GetTimer%20Seconds _asbp_third_person_game_mode) 5))
  (Audio|PlaySound2D "/Game/Static/Sounds/GameSFX/UIMisc_Feedback_36_up_CB_Sounddesign_ACTIVATION2.UIMisc_Feedback_36_up_CB_Sounddesign_ACTIVATION2" 1.0 (Math|Random|RandomFloatinRange 0.7 1.0) 0.0 0 0)
  (Actor|DestroyActor))

(event EventBeginPlay)

(event Collision|EventActorBeginOverlap
  (params (OtherActor :type Actor%20Object%20Reference)))

(event EventTick
  (params (DeltaSeconds :type Float%20%28single-precision%29)))

(fn ConstructionScript)